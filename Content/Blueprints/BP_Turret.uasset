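; BP_Turret is a twin-barrel turret that tracks the first BP_FPCharacter found at BeginPlay and fires BP_Projectile actors.
; Tick turns the turret in yaw only at a constant speed toward the target, with a 90-degree offset.
; A Delay on Tick paces shots by FireRate, and a toggle alternates the barrels.
; Projectiles spawn from barrel location alone, as the accuracy-based velocity logic is unconnected.
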(event `self.ReceiveBeginPlay`
  (bind _returnvalue (`GameplayStatics.GetActorOfClass` "/Game/Blueprints/Player/BP_FPCharacter.BP_FPCharacter_C"))
  (set `self.target` _returnvalue))

(event `self.ReceiveTick`
  (params (DeltaSeconds :type "Float (single-precision)"))
  (set `self.barrel1Pos` (`SceneComponent.K2_GetComponentLocation` (`self.barrel1`)))
  (set `self.barrel2Pos` (`SceneComponent.K2_GetComponentLocation` (`self.barrel2`)))
  (`self.Look At Target` DeltaSeconds)
  (`KismetSystemLibrary.Delay` (`self.fireRate`))
  (if (`self.barrelToggle`)
    (`self.Fire` (`self.barrel1Pos`))
    (else
      (`self.Fire` (`self.barrel2Pos`)))))

(fn `Fire`
  (params (Start :type "Vector Structure"))
  (locals (NewLocalVar :type Boolean))
  (bind _returnvalue (`|SpawnActorFromClass` "/Game/Blueprints/BP_Projectile.BP_Projectile_C" (`KismetMathLibrary.Conv_VectorToTransform` Start) "Undefined" "MultiplyWithRoot" null null))
  (set `self.barrelToggle` (not (`self.barrelToggle`))))

(fn `Look At Target`
  (params (`Delta Seconds` :type "Float (double-precision)"))
  (locals (targetPos :type "Vector Structure") (rotToTarget :type "Vector Structure"))
  (`SceneComponent.K2_SetWorldRotation` (`self.Turret`) (`KismetMathLibrary.RInterpTo_Constant` (`SceneComponent.K2_GetComponentRotation` (`self.Turret`)) (`KismetMathLibrary.MakeRotator` (.roll (`SceneComponent.K2_GetComponentRotation` (`self.Turret`))) (.pitch (`SceneComponent.K2_GetComponentRotation` (`self.Turret`))) (- (.yaw (`KismetMathLibrary.FindLookAtRotation` (`SceneComponent.K2_GetComponentLocation` (`self.Turret`)) (`self.K2_GetActorLocation` (`self.target`)))) 90.0)) (`local.Delta Seconds`) (`self.trackingSpeed`)) false false))

(fn `UserConstructionScript`)